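; BP_NorthPole is a placeable actor that defines compass north by writing a direction into the MPC_DirectionCoordinates material parameter collection.
; It sets the "North" parameter's R and G to the X and Y of the unit vector from the player camera toward itself.
; This runs every Tick or once at BeginPlay, depending on flags.
; Events toggle ticking or set north manually, and BeginPlay caches the initial value.
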(event Custom|Activate
  ;[1 1 1] Tick on/off
  (Actor|Tick|SetActorTickEnabled true))

(event Custom|Desactivate
  ;[1 1 1] Tick on/off
  (Actor|Tick|SetActorTickEnabled false))

(event Custom|SelfSetNorth
  (bind _returnvalue (Transformation|GetActorLocation))
  (bind _returnvalue_2 (Game|GetPlayerCameraManager 0))
  (bind _returnvalue_3 (Camera|GetCameraLocation _returnvalue_2))
  (bind _returnvalue_4 (Math|Vector|GetUnitDirection(Vector) _returnvalue_3 _returnvalue))
  ;[1 1 1] Set north auto / Manualy
  (Rendering|Material|SetVectorParameterValue "/Game/CompassAndMarkers/Sources/Blueprints/Compass/MPC_DirectionCoordinates.MPC_DirectionCoordinates" "North" (Utilities|Struct|MakeLinearColor (.x _returnvalue_4) (.y _returnvalue_4) 0.0 1.0) :!class /Script/Engine.KismetMaterialLibrary))

(event Custom|ManualSetNorth
  (params (Direction :type Vector))
  ;[1 1 1] Set north auto / Manualy
  (Rendering|Material|SetVectorParameterValue "/Game/CompassAndMarkers/Sources/Blueprints/Compass/MPC_DirectionCoordinates.MPC_DirectionCoordinates" "North" (Utilities|Struct|MakeLinearColor (.x Direction) (.y Direction) 0.0 1.0) :!class /Script/Engine.KismetMaterialLibrary))

(event EventTick
  (params (DeltaSeconds :type Float%20%28single-precision%29))
  (bind _returnvalue (Game|GetPlayerCameraManager 0))
  (bind _returnvalue_2 (Transformation|GetActorLocation))
  (bind _returnvalue_3 (Camera|GetCameraLocation _returnvalue))
  (bind _returnvalue_4 (Math|Vector|GetUnitDirection(Vector) _returnvalue_3 _returnvalue_2))
  ;[1 1 1] Tick
  (Rendering|Material|SetVectorParameterValue "/Game/CompassAndMarkers/Sources/Blueprints/Compass/MPC_DirectionCoordinates.MPC_DirectionCoordinates" "North" (Utilities|Struct|MakeLinearColor (.x _returnvalue_4) (.y _returnvalue_4) 0.0 1.0) :!class /Script/Engine.KismetMaterialLibrary))

(event EventBeginPlay
  ;[1 1 1] BeginPlay
  (bind _returnvalue (Rendering|Material|GetVectorParameterValue "/Game/CompassAndMarkers/Sources/Blueprints/Compass/MPC_DirectionCoordinates.MPC_DirectionCoordinates" "North" :!class /Script/Engine.KismetMaterialLibrary))
  (Variables|Default|SetInitialNorth _returnvalue)
  (if (Variables|Default|GetTick?)
    (CallFunction|Activate)
    (elif (Variables|Default|GetSetNorthOnBeginPlay)
      (CallFunction|SelfSetNorth))))

(fn ConstructionScript)