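; Map actor component that gives its owner a zoomable map capture.
; On BeginPlay it spawns a BP_MapCapture, attaches it to the owner and caches its render target and scene capture OrthoWidth.
; ZoomIn and ZoomOut change that OrthoWidth within clamped limits and write it back to the capture.
; Zooming out steps by the IncrPower variable, while zooming in uses a hardcoded step.
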(event Custom|ZoomOut
  ;[1 1 1] Zoom
  (bind _output_get (Variables|Default|SetOrtho%20Width (Math|Float|Clamp(Float) (+ (Variables|Default|GetOrtho%20Width) (Variables|Default|GetIncrPower)) 0.0 2.2e+03)))
  (Variables|/Script/Engine.SceneCaptureComponent2D|SetOrthoWidth (Variables|/Game/CompassAndMarkers/Sources/Blueprints/Map/BP_MapCapture.BP_MapCapture_C|GetMapSceneCapture (Variables|Default|GetSpawnedCapture)) _output_get))

(event Custom|ZoomIn
  ;[1 1 1] Zoom
  (bind _output_get (Variables|Default|SetOrtho%20Width (Math|Float|Clamp(Float) (- (Variables|Default|GetOrtho%20Width) 4e+02) 4.5e+02 2.2e+03)))
  (Variables|/Script/Engine.SceneCaptureComponent2D|SetOrthoWidth (Variables|/Game/CompassAndMarkers/Sources/Blueprints/Map/BP_MapCapture.BP_MapCapture_C|GetMapSceneCapture (Variables|Default|GetSpawnedCapture)) _output_get))

(event EventBeginPlay
  (bind _returnvalue (Components|GetOwner))
  ;[1 1 1] Init the map capture
  (bind _returnvalue_2 (Game|SpawnActorfromClass "/Game/CompassAndMarkers/Sources/Blueprints/Map/BP_MapCapture.BP_MapCapture_C" (Math|Transform|MakeTransform "0, 0, 0" "0, 0, 0" "1,1,1") "AlwaysSpawn" _returnvalue 0))
  (bind _output_get (Variables|Default|SetSpawnedCapture _returnvalue_2))
  (Transformation|AttachActorToActor _output_get _returnvalue "None" "KeepRelative" "KeepRelative" "KeepRelative" false)
  (Variables|Default|SetRTMap (Variables|/Game/CompassAndMarkers/Sources/Blueprints/Map/BP_MapCapture.BP_MapCapture_C|GetRTMap _returnvalue_2))
  (Variables|Default|SetOrtho%20Width (Variables|/Script/Engine.SceneCaptureComponent2D|GetOrthoWidth (Variables|/Game/CompassAndMarkers/Sources/Blueprints/Map/BP_MapCapture.BP_MapCapture_C|GetMapSceneCapture (Variables|Default|GetSpawnedCapture)))))