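; Scanner actor component that runs an expanding scan pulse and places markers on the "Discoverable" actors it reaches.
; StartScan sets up a hidden sphere at the owner and a camera modifier carrying a dynamic post-process material centred on the camera.
; A looping timer grows the sphere and material radius together until MaxRadius.
; Overlaps look up actor tags in a marker data table and call the player's BP_AC_Marker, using default markers for unmatched tags.
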(event Custom|StartScan
  (params (PosprocessMaterial :type Material%20Interface%20Object%20Reference) (Marker%20ID :type Integer))
  (bind _returnvalue (Components|GetOwner))
  (bind _returnvalue_2 (Transformation|GetActorLocation _returnvalue))
  ;[1 1 1] Start the scanning effect and timer
  (Variables|Default|SetMarker%20ID Marker%20ID)
  (Utilities|Map|Clear (Variables|Default|GetActorScanned))
  (Variables|Default|SetPosprocess%20Material PosprocessMaterial)
  (bind _sphere (Variables|Default|GetSphere)
    (:then
      (bind _output_get (Variables|Default|SetSphere _sphere))
      (Transformation|SetWorldLocation _output_get _returnvalue_2 false true))
    (:else
      (bind _returnvalue_3 (Game|AddComponentbyClass _returnvalue "/Script/Engine.SphereComponent" true (Math|Transform|MakeTransform _returnvalue_2 "0, 0, 0" "1,1,1")))
      (Variables|Default|SetSphere _returnvalue_3)))
  (Collision|SetCollisionResponsetoChannel (Variables|Default|GetSphere) "ECC_WorldDynamic" "ECR_Ignore")
  (Rendering|SetVisibility (Variables|Default|GetSphere) false true)
  (Development|SetHiddeninGame (Variables|Default|GetSphere) true true)
  (Variables|/Script/Engine.ActorComponent|SetComponentTags (Variables|Default|GetSphere) (Utilities|Array|MakeArray "Scan"))
  (Collision|SetCollisionObjectType (Variables|Default|GetSphere) "ECC_Visibility")
  (Utilities|FlowControl|DoOnce false
    (:Completed
      (Variables|Default|GetScanDynamicMaterial
        (:then
          _)
        (:else
          (bind _returnvalue_4 (Rendering|Material|CreateDynamicMaterialInstance (Variables|Default|GetPosprocess%20Material) "None" "None" :!class /Script/Engine.KismetMaterialLibrary))
          (Variables|Default|SetScanDynamicMaterial _returnvalue_4)))
      (Rendering|Material|SetVectorParameterValue (Variables|Default|GetScanDynamicMaterial) "ScanPos" (Math|Conversions|ToLinearColor(Vector) (Transformation|GetActorLocation (Game|GetPlayerCameraManager 0))) :!class /Script/Engine.MaterialInstanceDynamic)
      (bind _output_get_2 (Variables|Default|SetCurrentRadius 1.0))
      (Rendering|Material|SetScalarParameterValue (Variables|Default|GetScanDynamicMaterial) "Radius" _output_get_2 :!class /Script/Engine.MaterialInstanceDynamic)
      (bind _returnvalue_5 (Game|Player|AddNewCameraModifier (Game|GetPlayerCameraManager 0) "/Game/CompassAndMarkers/Sources/Blueprints/Scanner/BP_CM_ScanEffectModifier.BP_CM_ScanEffectModifier_C"))
      (Variables|Default|SetCameraModifier _returnvalue_5)
      (bind _returnvalue_6 (Utilities|Time|SetTimerbyEvent (delegate Custom|Timer) 0.022222 true))
      (Variables|Default|SetTimerScan _returnvalue_6)
      (bind _ascm_scan_effect_modifier (Utilities|Casting|CastToBP_CM_ScanEffectModifier (Variables|Default|GetCameraModifier)))
      (Variables|/Game/CompassAndMarkers/Sources/Blueprints/Scanner/BP_CM_ScanEffectModifier.BP_CM_ScanEffectModifier_C|SetScanEffectPostMat _ascm_scan_effect_modifier (Variables|Default|GetScanDynamicMaterial)))))

(event Custom|Timer
  ;[1 1 1] Check if overlapping hidden markers on timer
  (Collision|AssignOnComponentBeginOverlap (Variables|Default|GetSphere) (delegate Custom|OnComponentBeginOverlap_Event_0))
  (Rendering|Material|SetScalarParameterValue (Variables|Default|GetScanDynamicMaterial) "Radius" (+ (Variables|Default|GetCurrentRadius) (Variables|Default|GetExpendSpeed)) :!class /Script/Engine.MaterialInstanceDynamic)
  (bind _output_get (Variables|Default|SetCurrentRadius (+ (Variables|Default|GetCurrentRadius) (Variables|Default|GetExpendSpeed))))
  (Components|Sphere|SetSphereRadius (Variables|Default|GetSphere) (+ (Variables|Default|GetCurrentRadius) (Variables|Default|GetExpendSpeed)) true)
  (if (>= _output_get (Variables|Default|GetMaxRadius))
    (Utilities|Time|PauseTimerbyHandle (Variables|Default|GetTimerScan))
    (Utilities|FlowControl|Sequence
      (:then_0
        ;[1 1 1] Start the scanning effect and timer
        (Utilities|FlowControl|DoOnce false) ; enters at Reset
      )
      (:then_1
        (Game|Player|RemoveCameraModifier (Game|GetPlayerCameraManager 0) (Variables|Default|GetCameraModifier)))
      (:then_2
        (Components|Sphere|SetSphereRadius (Variables|Default|GetSphere) 0.0 false)))))

(event Custom|OnComponentBeginOverlap_Event_0
  (params (OverlappedComponent :type Primitive%20Component%20Object%20Reference) (OtherActor :type Actor%20Object%20Reference) (OtherComp :type Primitive%20Component%20Object%20Reference) (OtherBodyIndex :type Integer) (bFromSweep :type Boolean) (SweepResult :type Hit%20Result%20Structure%20%28by%20ref%29))
  (bind _returnvalue (Transformation|GetActorLocation OtherActor))
  (bind _marker_id (Variables|Default|GetMarker%20ID))
  ;[1 1 1] Check if overlapping hidden markers on timer
  (if (Actor|ActorHasTag OtherActor "Discoverable")
    (bind _array_element (Utilities|Array|ForEachLoopwithBreak (Variables|/Script/Engine.Actor|GetTags OtherActor) :!label _label)
      (:LoopBody
        (bind _returnvalue_2 (Utilities|GetDataTableRow "/Game/CompassAndMarkers/Sources/Blueprints/Markers/DT_MarkesDataTables.DT_MarkesDataTables" _array_element)
          (:then
            (goto _label Break))
          (:RowNotFound
            (Default|AddMarkeratLocation (Actor|GetComponentbyClass (Game|GetPlayerCharacter 0) "/Game/CompassAndMarkers/Sources/Blueprints/Markers/BP_AC_Marker.BP_AC_Marker_C") _marker_id _returnvalue "/Game/CompassAndMarkers/Sources/Blueprints/Markers/Default_Style/BP_Default_Marker.BP_Default_Marker_C"))))
      (:Completed
        (Default|AddMarkeratLocation (Actor|GetComponentbyClass (Game|GetPlayerCharacter 0) "/Game/CompassAndMarkers/Sources/Blueprints/Markers/BP_AC_Marker.BP_AC_Marker_C") _marker_id _returnvalue (.basemarkerbp _returnvalue_2))))))