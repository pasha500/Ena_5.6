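; Function library that scrolls a 2D compass strip as the player camera turns.
; Both functions set the "U" parameter on a retainer's effect material from normalized camera yaw, corrected by the North vector's angle in MPC_DirectionCoordinates.
; A half-segment shift is subtracted, with segment count taken from the grid's child count in the grid variant and from Offset in the image variant.
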(fn Compass2DGridTranslation
  (params (Grid :type Panel%20Widget%20Object%20Reference) (Retainer :type Retainer%20Box%20Object%20Reference))
  (bind _returnvalue (Math|Vector|MakeVector 1.0 0.0 0.0))
  (bind _returnvalue_2 (Rendering|Material|GetVectorParameterValue 0 "/Game/CompassAndMarkers/Sources/Blueprints/Compass/MPC_DirectionCoordinates.MPC_DirectionCoordinates" "North" :!class /Script/Engine.KismetMaterialLibrary))
  (Rendering|Material|SetScalarParameterValue (Class|RetainerBox|GetEffectMaterial Retainer) "U" (+ (Math|Float|NormalizetoRange (.Yaw (Math|Rotator|BreakRotator (Camera|GetCameraRotation (Game|GetPlayerCameraManager 0)))) 0.0 3.6e+02) (Math|Float|NormalizetoRange (- (* (- (Class|KismetMathLibrary|DegAtan2 (.x _returnvalue) (.y _returnvalue)) (Class|KismetMathLibrary|DegAtan2 (.x (Math|Vector|MakeVector (.r _returnvalue_2) (.g _returnvalue_2) 0.0)) (.y (Math|Vector|MakeVector (.r _returnvalue_2) (.g _returnvalue_2) 0.0)))) -1.0) (/ 3.6e+02 (Math|Conversions|ToFloat(Integer) (* (Utilities|Array|Length (Class|PanelWidget|GetAllChildren Grid)) 2)))) 0.0 3.6e+02)) :!class /Script/Engine.MaterialInstanceDynamic))

(fn Compass2DImageTranslation
  (params (Retainer :type Retainer%20Box%20Object%20Reference) (Offset :type Float%20%28single-precision%29))
  (bind _returnvalue (Math|Vector|MakeVector 1.0 0.0 0.0))
  (bind _returnvalue_2 (Rendering|Material|GetVectorParameterValue 0 "/Game/CompassAndMarkers/Sources/Blueprints/Compass/MPC_DirectionCoordinates.MPC_DirectionCoordinates" "North" :!class /Script/Engine.KismetMaterialLibrary))
  (Rendering|Material|SetScalarParameterValue (Class|RetainerBox|GetEffectMaterial Retainer) "U" (+ (Math|Float|NormalizetoRange (.Yaw (Math|Rotator|BreakRotator (Camera|GetCameraRotation (Game|GetPlayerCameraManager 0)))) 0.0 3.6e+02) (Math|Float|NormalizetoRange (- (* (- (Class|KismetMathLibrary|DegAtan2 (.x _returnvalue) (.y _returnvalue)) (Class|KismetMathLibrary|DegAtan2 (.x (Math|Vector|MakeVector (.r _returnvalue_2) (.g _returnvalue_2) 0.0)) (.y (Math|Vector|MakeVector (.r _returnvalue_2) (.g _returnvalue_2) 0.0)))) -1.0) (/ 3.6e+02 (* Offset 2.0))) 0.0 3.6e+02)) :!class /Script/Engine.MaterialInstanceDynamic))