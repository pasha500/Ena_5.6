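; Base world marker actor that shows itself on the compass bar, map and as a screen-edge indicator.
; On spawn it filters by team ID and spam limit, creates overridable widgets and registers with the compass bar.
; A looping timer updates distance text and height-difference state via render opacity.
; Tick clamps the off-screen indicator to viewport edges, including behind-camera cases, adjusts tick rate and yaws the map widget with the map capture.
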(event Custom|UpdateTimer
  (bind _returnvalue (Transformation|GetActorLocation))
  (bind _returnvalue_2 (Game|Player|GetPlayerPawn 0))
  (bind _returnvalue_3 (Transformation|GetActorLocation _returnvalue_2))
  ;[1 1 1] Update distance + height timer then send it to the widget
  (Utilities|IsValid (Game|GetPlayerCharacter 0)
    (:Is%20Valid
      (bind _markerwidget (Variables|Default|GetMarkerWidget)
        (:then
          (if (<= (Math|Float|Absolute(Float) (- (.z _returnvalue_3) (.z _returnvalue))) (Variables|Default|GetHeightToleranceCheck))
            (Widget|SetRenderOpacity _markerwidget 1.0)
            (else
              (Math|Float|CompareFloat (.z _returnvalue_3) (.z _returnvalue)
                (:>
                  (Widget|SetRenderOpacity _markerwidget 3.0))
                (:<
                  (Widget|SetRenderOpacity _markerwidget 2.0)))))
          (if (> (Math|Vector|VectorLength (Transformation|GetVelocity (Game|GetPlayerCharacter 0))) 0.0)
            (bind _markerwidget_2 (Variables|Default|GetMarkerWidget)
              (:then
                (Class|Widget|SetToolTipText _markerwidget_2 (Utilities|Text|ToText(Integer) (Math|Float|Truncate (/ (Math|Vector|Distance(Vector) (Transformation|GetActorLocation) (Transformation|GetActorLocation (Game|Player|GetPlayerPawn 0))) 1e+02)))))
              (:else))))
        (:else)))))

(event Custom|Spawned
  ;[1 1 1] begin
  ;;[1 1 1] Init serverside
  (Networking|SwitchHasAuthority
    (:Authority
      (CallFunction|BeginAll))))

(event Custom|DestroyOnClient
  ;[1 1 1] begin
  ;;[1 1 1] runing on client
  (Rendering|SetActorHiddenInGame true)
  (Actor|DestroyActor))

(event Custom|RPCAddmarkerclient
  (params (MarkerWidget :type Widget%20Object%20Reference) (MarkerBP :type BP%20Base%20Marker%20Object%20Reference) (HeightToleranceCheck :type Float%20%28single-precision%29))
  ;[1 1 1] Add to compass
  (Utilities|CheckTeam
    (:Pass
      (Utilities|IsValid (Variables|/Game/CompassAndMarkers/Sources/Blueprints/Compass/BP_AC_CompassBar.BP_AC_CompassBar_C|GetCompassWidget (Actor|GetComponentbyClass (Pawn|GetControlledPawn (Game|GetPlayerController 0)) "/Game/CompassAndMarkers/Sources/Blueprints/Compass/BP_AC_CompassBar.BP_AC_CompassBar_C"))
        (:Is%20Valid
          (Default|Addclientmulti (Variables|Default|GetCompassBarMarker) (Variables|Default|GetCompassWidget) MarkerBP HeightToleranceCheck)
          ;[1 1 1] Sound
          (CallFunction|PlaySound (Variables|Default|GetSoundLocation)))))))

(event Custom|TeamOnClient
  ;[1 1 1] begin
  ;;[1 1 1] runing on client
  (Utilities|CheckTeam
    (:Pass
      (Rendering|SetActorHiddenInGame false))
    (:DontPass
      (Rendering|SetActorHiddenInGame true)
      (Actor|DestroyActor))))

(event Custom|RunOnServer
  ;[1 1 1] begin
  ;;[1 1 1] runing on server
  (Utilities|CheckTeam
    (:Pass
      (Rendering|SetActorHiddenInGame false))
    (:DontPass
      (Class|PrimitiveComponent|SetOwnerNoSee (Variables|Default|GetMarker) true))))

(event Custom|SpwanedClientSide
  ;[1 1 1] begin
  ;;[1 1 1] Init client side
  (Networking|SwitchHasAuthority
    (:Authority
      (Utilities|CheckTeam
        (:Pass
          (Rendering|SetActorHiddenInGame false))
        (:DontPass
          (Widget|SetVisibility (UserInterface|GetWidget (Variables|Default|GetMarker)) "Hidden"))))))

(event Custom|BeginAll
  (bind _returnvalue (Transformation|GetActorLocation))
  (bind _returnvalue_2 (Game|Player|GetPlayerPawn 0))
  (bind _returnvalue_3 (Transformation|GetActorLocation _returnvalue_2))
  ;[1 1 1] begin
  (bind _outactors (Actor|GetAllActorsOfClass (Utilities|GetClass self)))
  (if (== (Variables|Default|GetMarkerSpamLimit) 0)
    (CallFunction|TeamonClient :!label _label)
    (Utilities|FlowControl|Sequence
      (:then_0
        (Utilities|Time|SetTimerbyEvent (delegate Custom|UpdateTimer) 0.2 true))
      (:then_1
        (bind _foundwidgets (Widget|GetAllWidgetsOfClass "/Game/CompassAndMarkers/Sources/Blueprints/Compass/WBP_CompassBarMarkers.WBP_CompassBarMarkers_C" false))
        (bind _output_get (Variables|Default|SetCompassBarMarker (Utilities|Array|Get(acopy) _foundwidgets (Utilities|Array|LastIndex _foundwidgets))))
        (if (== _output_get 0)
          (bind _foundwidgets_2 (Widget|GetAllWidgetsOfClass "/Game/CompassAndMarkers/Sources/Blueprints/Compass/WBP_CompassBarMarkers.WBP_CompassBarMarkers_C" false))
          (Utilities|FlowControl|Delay 0.02)
          (Variables|Default|SetCompassBarMarker (Utilities|Array|Get(acopy) _foundwidgets_2 (Utilities|Array|LastIndex _foundwidgets_2))))
        (if (Networking|IsDedicatedServer)
          (Networking|SwitchHasAuthority
            (:Authority
              _)
            (:Remote
              ;[1 1 1] Off screen widget support
              (if (Variables|Default|GetOffScreenIndicator) :!label _label_2
                (bind _returnvalue_4 (UserInterface|CreateWidget (Variables|Default|GetOffScreenWidget_Owerride) (Game|GetPlayerController 0)))
                (Variables|Default|SetOffScreenWiget _returnvalue_4)
                (Utilities|CheckTeam
                  (:Pass
                    (UserInterface|Viewport|AddtoViewport (Variables|Default|GetOffScreenWiget) 0)
                    (Variables|Default|SetOffSInitialDesiredSize (Class|Widget|GetDesiredSize (Variables|Default|GetOffScreenWiget)))
                    (Widget|SetVisibility (Variables|Default|GetOffScreenWiget) "Collapsed"))
                  (:DontPass
                    _)))
              ;[1 1 1] Main Widgets Setup
              (Class|PrimitiveComponent|SetVisibleinSceneCaptureOnly (Variables|Default|GetTopWidget) true)
              (bind _returnvalue_5 (UserInterface|CreateWidget (Variables|Default|GetDefaultWidget) (Game|GetPlayerController 0)))
              (bind _output_get_2 (Variables|Default|SetMarkerWidget _returnvalue_5))
              (Class|Widget|SetToolTipText _output_get_2 (Utilities|Text|ToText(Integer) (Math|Float|Truncate (/ (Math|Vector|Distance(Vector) (Transformation|GetActorLocation) (Transformation|GetActorLocation (Game|Player|GetPlayerPawn 0))) 1e+02))))
              (UserInterface|SetWidget (Variables|Default|GetTopWidget) _output_get_2)
              (UserInterface|SetWidget (Variables|Default|GetMarker) _output_get_2)
              (bind _returnvalue_6 (UserInterface|CreateWidget (Variables|Default|GetCompassWidget_Override) (Game|GetPlayerController 0)))
              (Variables|Default|SetCompassWidget _returnvalue_6)
              (Class|Widget|SetToolTipText (Variables|Default|GetMarkerWidget) (Utilities|Text|ToText(Integer) (Math|Float|Truncate (/ (Math|Vector|Distance(Vector) (Transformation|GetActorLocation) (Transformation|GetActorLocation (Game|Player|GetPlayerPawn 0))) 1e+02))))
              (bind _returnvalue_7 (UserInterface|CreateWidget (Variables|Default|GetMapWidget_Override) (Game|GetPlayerController 0)))
              (bind _output_get_3 (Variables|Default|SetMapWidget _returnvalue_7))
              (UserInterface|SetWidget (Variables|Default|GetTopWidget) _output_get_3)))
          (else
            (goto _label_2)))
        ;[1 1 1] Add to compass
        (Networking|SwitchHasAuthority
          (:Authority
            (CallFunction|RPCAddmarkerclient (Variables|Default|GetMarkerWidget) self (Variables|Default|GetHeightToleranceCheck)))))
      (:then_2
        ;[1 1 1] Update distance + height timer then send it to the widget
        (Utilities|IsValid (Game|GetPlayerCharacter 0)
          (:Is%20Valid
            (Utilities|FlowControl|DoOnce false
              (:Completed
                (bind _markerwidget (Variables|Default|GetMarkerWidget :!label _label_3)
                  (:then
                    (Class|Widget|SetToolTipText _markerwidget (Utilities|Text|ToText(Integer) (Math|Float|Truncate (/ (Math|Vector|Distance(Vector) (Transformation|GetActorLocation) (Transformation|GetActorLocation (Game|Player|GetPlayerPawn 0))) 1e+02)))))
                  (:else)))))))
      (:then_3
        (Utilities|IsValid (Game|GetPlayerCharacter 0)
          (:Is%20Valid
            (bind _markerwidget_2 (Variables|Default|GetMarkerWidget)
              (:then
                (if (<= (Math|Float|Absolute(Float) (- (.z _returnvalue_3) (.z _returnvalue))) (Variables|Default|GetHeightToleranceCheck))
                  (Widget|SetRenderOpacity _markerwidget_2 1.0)
                  (else
                    (Math|Float|CompareFloat (.z _returnvalue_3) (.z _returnvalue)
                      (:>
                        (Widget|SetRenderOpacity _markerwidget_2 3.0))
                      (:<
                        (Widget|SetRenderOpacity _markerwidget_2 2.0)))))
                (if (> (Math|Vector|VectorLength (Transformation|GetVelocity (Game|GetPlayerCharacter 0))) 0.0)
                  (goto _label_3)))
              (:else)))))
      (:then_4
        (Variables|Default|SetTopWidgetInitPos (Transformation|GetWorldRotation (Variables|Default|GetTopWidget)))))
    (elif (< (- (Utilities|Array|Length _outactors) 1) (Variables|Default|GetMarkerSpamLimit))
      (goto _label)
      (else
        (CallFunction|DestroyonClient)))))

(event EventTick
  (params (DeltaSeconds :type Float%20%28single-precision%29))
  (bind _returnvalue (Game|Player|GetPlayerPawn 0))
  (bind _offscreenwiget (Variables|Default|GetOffScreenWiget))
  (bind _topwidgetinitpos (Variables|Default|GetTopWidgetInitPos))
  (bind _returnvalue_2 (Actor|GetComponentbyClass _returnvalue "/Game/CompassAndMarkers/Sources/Blueprints/Map/BP_AC_Map.BP_AC_Map_C"))
  (bind _spawnedcapture (Variables|/Game/CompassAndMarkers/Sources/Blueprints/Map/BP_AC_Map.BP_AC_Map_C|GetSpawnedCapture _returnvalue_2))
  ;[1 0 0] tick
  (Utilities|IsValid _offscreenwiget
    (:Is%20Valid
      (if (not (== _offscreenwiget 0))
        (CallFunction|OffScreen)
        (if (Utilities|IsValid _spawnedcapture)
          (Utilities|FlowControl|FlipFlop
            (:A
              (Transformation|SetWorldRotation (Variables|Default|GetTopWidget) (Math|Rotator|MakeRotator (.roll _topwidgetinitpos) (.pitch _topwidgetinitpos) (.yaw (Transformation|GetActorRotation _spawnedcapture))) false false))))))))

(event EventDestroyed
  (bind _compasswidget (Variables|Default|GetCompassWidget))
  ;[0 0.9519 1] On Destroy
  (if (Utilities|IsValid _compasswidget)
    (Utilities|IsValid (Variables|Default|GetCompassBarMarker)
      (:Is%20Valid
        (Default|RemoveMarkeronCompass (Variables|Default|GetCompassBarMarker) self _compasswidget)
        (Widget|RemovefromParent (Variables|Default|GetOffScreenWiget))))))

(fn ConstructionScript
  ;[1 1 1] Setup base widget if none
  (Transformation|AddWorldOffset (Variables|Default|GetDefaultSceneRoot) (Variables|Default|GetWorldOffset) false false)
  (Variables|Default|GetDefaultWidget
    (:then
      _)
    (:else
      (Development|PrintString "Error: DefaultWidget not specified" true true "(R=1.000000,G=0.007073,B=0.000000,A=1.000000)")
      (Variables|Default|SetDefaultWidget "/Game/CompassAndMarkers/Sources/Blueprints/Markers/WBP_Default_Marker2D.WBP_Default_Marker2D_C")))
  (Variables|Default|GetMapWidget_Override
    (:then
      _)
    (:else
      (Variables|Default|SetMapWidget_Override (Variables|Default|GetDefaultWidget))))
  (Variables|Default|GetOffScreenWidget_Owerride
    (:then
      _)
    (:else
      (Variables|Default|SetOffScreenWidget_Owerride (Variables|Default|GetDefaultWidget))))
  (Variables|Default|GetCompassWidget_Override
    (:then)
    (:else
      (Variables|Default|SetCompassWidget_Override (Variables|Default|GetDefaultWidget))
      (Rendering|SetVisibility (Variables|Default|GetDefaultSceneRoot) true false)
      (if (not (Variables|Default|GetAddToMap))
        (Transformation|SetActorScale3D "0, 0, 0")))))

(fn PlaySound
  (params (Location :type Vector))
  ;[1 1 1] Play sound 2D is marker location is 0
  (Variables|Default|GetSound
    (:then
      (if (Math|Vector|Equal(Vector) Location "0, 0, 0" 0.0001)
        (Audio|PlaySound2D (Variables|Default|GetSound) 1.0 1.0 0.0 0 0)
        (else
          (Audio|PlaySoundatLocation (Variables|Default|GetSound) (Variables|Default|GetSoundLocation) "0, 0, 0" 1.0 1.0 0.0 0 0 0))))
    (:else)))

(fn OffScreen
  (bind _returnvalue (Game|GetPlayerController 0))
  (bind _returnvalue_2 (Game|GetPlayerController 0))
  (bind _returnvalue_3 (Game|GetPlayerController 0))
  (bind _returnvalue_4 (Viewport|GetViewportSize))
  (bind _returnvalue_5 (Viewport|GetViewportSize))
  (bind _returnvalue_6 (Transformation|GetActorLocation))
  (bind _returnvalue_7 (Viewport|GetViewportSize))
  (bind _returnvalue_8 (Game|GetPlayerCameraManager 0))
  (bind _self self)
  (bind _self_2 self)
  (bind _returnvalue_9 (Camera|GetCameraLocation _returnvalue_8))
  (bind _returnvalue_10 (Transformation|GetActorLocation _self))
  (bind _returnvalue_11 (Transformation|GetActorLocation _self_2))
  (bind (_screenposition _returnvalue_12) (Class|GameplayStatics|ProjectWorldtoScreen _returnvalue_3 _returnvalue_6 true))
  (bind (_screenposition_2 _returnvalue_13) (Class|GameplayStatics|ProjectWorldtoScreen _returnvalue_2 (Math|Vector|MakeVector (.x _returnvalue_10) (.y _returnvalue_10) (.z _returnvalue_10)) true))
  (bind _returnvalue_14 (- _returnvalue_9 _returnvalue_11))
  (bind _returnvalue_15 (Math|Vector|Normalize _returnvalue_14))
  (bind _returnvalue_16 (* _returnvalue_15 5e+03))
  (bind _returnvalue_17 (+ _returnvalue_9 _returnvalue_16))
  (bind _screenposition_3 (Class|GameplayStatics|ProjectWorldtoScreen _returnvalue (Math|Vector|MakeVector (.x _returnvalue_17) (.y _returnvalue_17) 2e+03) true))
  (bind (_offscreen _xpos _ypos) (Utilities|OffscreenPositionifBehind (.x _returnvalue_17) (.y _returnvalue_17)))
  (if (Variables|/Script/Engine.SceneComponent|GetbVisible (Variables|Default|GetDefaultSceneRoot))
    (Utilities|IsValid (Variables|Default|GetOffScreenWiget)
      (:Is%20Valid
        (if (Math|Boolean|ORBoolean (> (.x _screenposition) (.x _returnvalue_7)) (> (.y _screenposition) (.y _returnvalue_7)) (< (.x _screenposition) 0.0) (< (.y _screenposition) 0.0) (not _returnvalue_12))
          ;[1 0.4896 0.4896] Optimise tickrate
          (Actor|Tick|SetActorTickInterval 0.0)
          (Utilities|FlowControl|Sequence
            (:then_0
              (Utilities|FlowControl|DoOnce false :!label _label
                (:Completed
                  (Widget|SetVisibility (Variables|Default|GetOffScreenWiget) "Visible")
                  (Variables|Default|SetOffSInitialDesiredSize (Class|Widget|GetDesiredSize (Variables|Default|GetOffScreenWiget)))
                  (Class|UserWidget|SetAlignmentinViewport (Variables|Default|GetOffScreenWiget) "(X=0.500000,Y=0.500000)")
                  (goto _label_2 Reset))))
            (:then_1
              ;[1 1 1] Offscreen position if not behind
              (if _returnvalue_13
                (Class|UserWidget|SetPositioninViewport (Variables|Default|GetOffScreenWiget) (Math|Vector2D|MakeVector2D (Math|Float|Clamp(Float) (.x _screenposition_2) (+ 0.0 (+ (/ (Math|Float|Absolute(Float) (.x (Variables|Default|GetOffSInitialDesiredSize))) 2.0) (Variables|Default|GetOffScreenPadding))) (- (.x _returnvalue_4) (+ (/ (Math|Float|Absolute(Float) (.x (Variables|Default|GetOffSInitialDesiredSize))) 2.0) (Variables|Default|GetOffScreenPadding)))) (Math|Float|Clamp(Float) (.y _screenposition_2) (+ 0.0 (+ (/ (Math|Float|Absolute(Float) (.y (Variables|Default|GetOffSInitialDesiredSize))) 2.0) (Variables|Default|GetOffScreenPadding))) (- (.y _returnvalue_4) (+ (/ (Math|Float|Absolute(Float) (.y (Variables|Default|GetOffSInitialDesiredSize))) 2.0) (Variables|Default|GetOffScreenPadding))))) true)
                (Utilities|FlowControl|FlipFlop ; 1/2 frames
                  (:A
                    (Class|Widget|SetRenderTransformAngle (Variables|Default|GetOffScreenWiget) (Utilities|FindAngleOffscreen))))
                (else
                  ;[1 1 1] Offscreen pos if behind
                  (if _offscreen
                    (Class|UserWidget|SetPositioninViewport (Variables|Default|GetOffScreenWiget) (Math|Vector2D|MakeVector2D _xpos _ypos) true)
                    (Utilities|FlowControl|FlipFlop ; 1/2 frames
                      (:A
                        ;[1 1 1] Offscreen angle corection
                        (Class|Widget|SetRenderTransformAngle (Variables|Default|GetOffScreenWiget) (+ (Math|Rotator|NormalizeAxis (.yaw (Math|Rotator|FindLookatRotation (Math|Vector|MakeVector (.x _screenposition_3) (.y _screenposition_3) 0.0) (Math|Vector|MakeVector (.x (/ _returnvalue_5 2.0)) (.Y (Math|Vector2D|BreakVector2D _returnvalue_5)) 0.0)))) 1.8e+02)))))))))
          (else
            (Actor|Tick|SetActorTickInterval 0.1)
            (if (Widget|IsVisible (Variables|Default|GetOffScreenWiget))
              (Utilities|FlowControl|DoOnce false :!label _label_2
                (:Completed
                  (Utilities|FlowControl|Sequence
                    (:then_0
                      (goto _label Reset))
                    (:then_1
                      (Widget|SetVisibility (Variables|Default|GetOffScreenWiget) "Collapsed"))))))))))))