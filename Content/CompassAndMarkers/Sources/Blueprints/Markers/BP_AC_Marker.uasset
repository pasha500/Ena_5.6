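; Marker component that places world markers at the point the local camera looks at, or at a given location.
; A camera line trace reads the hit actor's tags to pick a marker class from DT_MarkesDataTables, falling back to BP_Default_Marker.
; SpawnOnserver spawns and initializes the marker, skips actors whose "marker" socket exists and that already carry one, and can attach it to the hit actor.
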(event Custom|AddMarkerInLine
  (params (MarkerID :type Integer) (Distance :type Float%20%28single-precision%29) (AttachToActor :type Boolean))
  (bind _returnvalue (Game|GetPlayerController 0))
  (bind _returnvalue_2 (Game|GetPlayerCameraManager 0))
  (bind _transformcomponent (Variables|/Script/Engine.PlayerCameraManager|GetTransformComponent _returnvalue_2))
  (bind _returnvalue_3 (Transformation|GetWorldLocation _transformcomponent))
  ;[1 0 0.9278] Linestrace - Spawn Marker - Set the widegt class - Check if attached
  (Variables|Default|SetAttach%20to%20Actor AttachToActor)
  (Variables|Default|SetMarker%20ID MarkerID)
  (Variables|Default|SetLocalPlayerController (Game|GetPlayerController 0))
  (bind _outhit (Collision|LineTraceByChannel _returnvalue_3 (+ _returnvalue_3 (* (Transformation|GetActorForwardVector _returnvalue_2) (Math|Float|SelectFloat (Variables|Default|GetDistance) Distance (<= Distance 0.0)))) "TraceTypeQuery1" true 0 "None"))
  (if (.bblockinghit _outhit)
    (Variables|Default|SetOut%20Hit%20Hit%20Actor (.hitactor _outhit))
    (Variables|Default|SetLocalOut%20Hit%20Location (.location _outhit))
    (if (<= (Utilities|Array|Length (Variables|/Script/Engine.Actor|GetTags (.hitactor _outhit))) 0)
      (Variables|Default|SetBaseMarkerClass "/Game/CompassAndMarkers/Sources/Blueprints/Markers/Default_Style/BP_Default_Marker.BP_Default_Marker_C" :!label _label)
      (else
        (bind _array_element (Utilities|Array|ForEachLoopwithBreak (Variables|/Script/Engine.Actor|GetTags (.hitactor _outhit)) :!label _label_2)
          (:LoopBody
            (Utilities|GetDataTableRow "/Game/CompassAndMarkers/Sources/Blueprints/Markers/DT_MarkesDataTables.DT_MarkesDataTables" _array_element
              (:then
                (goto _label_2 Break))))
          (:Completed
            (bind _returnvalue_4 (Utilities|GetDataTableRow "/Game/CompassAndMarkers/Sources/Blueprints/Markers/DT_MarkesDataTables.DT_MarkesDataTables" _array_element)
              (:then
                (Variables|Default|SetBaseMarkerClass (.basemarkerbp _returnvalue_4)))
              (:RowNotFound
                (goto _label)))))))
    (CallFunction|SpawnOnserver (Variables|Default|GetLocalOut%20Hit%20Location) _returnvalue _returnvalue (Variables|Default|GetBaseMarkerClass) (Variables|Default|GetMarker%20ID) (Variables|Default|GetOut%20Hit%20Hit%20Actor))))

(event Custom|AddMarkerAtLocation
  (params (Marker%20ID :type Integer) (MarkeWorldLocation :type Vector) (MarkerToAdd :type BP%20Base%20Marker%20Class%20Reference))
  (bind _returnvalue (Game|GetPlayerController 0))
  ;[1 0 0.9278] Add at Location
  (Variables|Default|SetAttach%20to%20Actor false)
  (Variables|Default|SetMarker%20ID Marker%20ID)
  (Variables|Default|SetBaseMarkerClass MarkerToAdd)
  (Variables|Default|SetLocalOut%20Hit%20Location MarkeWorldLocation)
  ;[1 0 0.9278] Linestrace - Spawn Marker - Set the widegt class - Check if attached
  (CallFunction|SpawnOnserver (Variables|Default|GetLocalOut%20Hit%20Location) _returnvalue _returnvalue (Variables|Default|GetBaseMarkerClass) (Variables|Default|GetMarker%20ID) (Variables|Default|GetOut%20Hit%20Hit%20Actor)))

(event Custom|SpawnOnserver
  (params (Spawn%20Transform%20Location :type Vector) (Owner :type Actor%20Object%20Reference) (OwnerPlayerController :type Player%20Controller%20Object%20Reference) (Class :type Actor%20Class%20Reference) (MarkerID :type Integer) (Out%20Hit%20Hit%20Actor :type Actor%20Object%20Reference))
  ;[1 0 0.9278] Linestrace - Spawn Marker - Set the widegt class - Check if attached
  (Utilities|IsValid Out%20Hit%20Hit%20Actor
    (:Is%20Valid
      (if (Transformation|DoesSocketExist (Variables|/Script/Engine.Actor|GetRootComponent Out%20Hit%20Hit%20Actor) "marker")
        (bind _filteredarray (Utilities|Array|FilterArray (Actor|GetAttachedActors Out%20Hit%20Hit%20Actor true) "/Game/CompassAndMarkers/Sources/Blueprints/Markers/BP_Base_Marker.BP_Base_Marker_C"))
        (if (not (> (Utilities|Array|Length _filteredarray) 0))
          (bind _returnvalue (Game|SpawnActorfromClass Class (Math|Transform|MakeTransform Spawn%20Transform%20Location "0, 0, 0" "1,1,1") "Undefined" Owner 0 :!label _label))
          (Variables|Default|SetSpawnedActor _returnvalue)
          (bind _asbp_base_marker (Utilities|Casting|CastToBP_Base_Marker _returnvalue))
          (bind _output_get (Variables|Default|SetAs%20BP%20Base%20Marker _asbp_base_marker))
          (Variables|/Game/CompassAndMarkers/Sources/Blueprints/Markers/BP_Base_Marker.BP_Base_Marker_C|SetMarkerID _output_get MarkerID)
          (if (Variables|Default|GetAttach%20to%20Actor)
            (if (Transformation|DoesSocketExist (Variables|/Script/Engine.Actor|GetRootComponent Out%20Hit%20Hit%20Actor) "marker")
              (Transformation|AttachActorToActor (Variables|Default|GetSpawnedActor) Out%20Hit%20Hit%20Actor "marker" "SnapToTarget" "SnapToTarget" "SnapToTarget" true)
              (else
                (Transformation|AttachActorToActor (Variables|Default|GetSpawnedActor) Out%20Hit%20Hit%20Actor "Marker" "KeepWorld" "KeepWorld" "KeepWorld" true))))
          (Default|Spawned (Variables|Default|GetAs%20BP%20Base%20Marker))
          (bind _as_bp_base_marker (Variables|Default|GetAs%20BP%20Base%20Marker)
            (:then
              (Default|SpwanedClientSide _as_bp_base_marker))
            (:else)))
        (else
          (goto _label))))
    (:Is%20Not%20Valid
      (goto _label))))

(event EventBeginPlay
  ;[1 1 1] begin play - Seting player
  (Variables|Default|SetLocalPlayerController (Game|GetPlayerController 0)))