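; BP_AC_CompassBar is a component that shows and hides the compass bar widget on the player's screen.
; AddCompassWidget stores the given widget class, then creates a fresh widget for player controller 0, adds it to the player screen and records the on-screen state.
; A DoOnce blocks repeated adds until RemoveCompassWidget removes the widget, clears that state and resets the gate.
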(event Custom|AddCompassWidget
  (params (CompassClass :type User%20Widget%20Class%20Reference))
  ;[1 1 1] add and remove widget on screen
  (Variables|Default|SetCompassClass CompassClass)
  (Utilities|FlowControl|DoOnce false
    (:Completed
      (bind _compasswidget (Variables|Default|GetCompassWidget)
        (:then
          (if (not (Variables|Default|GetOnScreen))
            (Widget|RemovefromParent _compasswidget)
            (bind _returnvalue (UserInterface|CreateWidget (Variables|Default|GetCompassClass) (Game|GetPlayerController 0) :!label _label))
            (bind _output_get (Variables|Default|SetCompassWidget _returnvalue))
            (bind _returnvalue_2 (UserInterface|Viewport|AddtoPlayerScreen _output_get))
            (Variables|Default|SetOnScreen _returnvalue_2)))
        (:else
          (goto _label))))))

(event Custom|RemoveCompassWidget
  ;[1 1 1] add and remove widget on screen
  (bind _compasswidget (Variables|Default|GetCompassWidget)
    (:then
      (Widget|RemovefromParent _compasswidget))
    (:else
      _))
  (Variables|Default|SetOnScreen false)
  (Utilities|FlowControl|DoOnce false) ; enters at Reset
)